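; Enemy character that chases the player, deals melee damage and pays out coins when shot dead.
; BeginPlay randomizes mesh scale and walk speed for variety.
; Pawn sensing triggers an AI move to the player, applying damage and a punch sound on arrival.
; Projectile hits subtract the player's gun damage; at zero health it ragdolls, awards coins and is destroyed after a delay, while CallDeath offers a shorter, reward-free death.
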(event OnSeePawn(PawnSensing)
  (params (Pawn :type Pawn%20Object%20Reference))
  (bind _self self)
  ;[1 1 1] Move To Player
  (bind _asfirst_person_character (Utilities|Casting|CastToFirstPersonCharacter Pawn))
  (Utilities|FlowControl|Delay 0.2)
  (AI|AIMoveTo _self "0, 0, 0" _asfirst_person_character 5.0 false
    (:OnSuccess
      (Game|Damage|ApplyDamage _asfirst_person_character (Variables|Default|GetDamageDone) 0 _self)
      (Audio|PlaySound2D "/Game/Sounds/Punch/PunchQueue.PunchQueue" 1.0 1.0 0.0 0 0))))

(event Custom|CallDeath
  (Physics|SetSimulatePhysics (Variables|Character|GetMesh) true)
  (Audio|PlaySound2D "/Game/Sounds/Bonedeath/bONEdEATHSound.bONEdEATHSound" 1.0 1.0 0.0 0 0)
  (Utilities|FlowControl|Delay 2.0)
  (Actor|DestroyActor))

(event EventBeginPlay
  (bind _returnvalue (Math|Random|RandomFloatinRange 0.9 1.2))
  ;[1 1 1] Randomize enemy
  (Transformation|SetWorldScale3D (Variables|Character|GetMesh) (Math|Vector|MakeVector _returnvalue _returnvalue _returnvalue))
  (Variables|/Script/Engine.CharacterMovementComponent|SetMaxWalkSpeed (Variables|Character|GetCharacterMovement) (Math|Random|RandomFloatinRange 5.5e+02 9.5e+02)))

(event Collision|EventHit
  (params (MyComp :type Primitive%20Component%20Object%20Reference) (Other :type Actor%20Object%20Reference) (OtherComp :type Primitive%20Component%20Object%20Reference) (bSelfMoved :type Boolean) (HitLocation :type Vector :default "0, 0, 0") (HitNormal :type Vector :default "0, 0, 0") (NormalImpulse :type Vector :default "0, 0, 0") (Hit :type Hit%20Result%20Structure%20%28by%20ref%29))
  ;[1 1 1] Getting Hit By Projectile
  (bind _asfirst_person_projectile (Utilities|Casting|CastToFirstPersonProjectile Other))
  (bind _asfirst_person_character (Utilities|Casting|CastToFirstPersonCharacter (Game|GetPlayerCharacter 0)))
  (Variables|Default|SetHealth (- (Variables|Default|GetHealth) (Variables|/Game/FirstPersonBP/Blueprints/FirstPersonCharacter.FirstPersonCharacter_C|GetGunDamage _asfirst_person_character)))
  (if (<= (Variables|Default|GetHealth) 0.0)
    (Physics|SetSimulatePhysics (Variables|Character|GetMesh) true)
    (Actor|DestroyActor _asfirst_person_projectile)
    (Audio|PlaySound2D "/Game/Sounds/Bonedeath/bONEdEATHSound.bONEdEATHSound" 1.0 1.0 0.0 0 0)
    (bind _asfirst_person_character_2 (Utilities|Casting|CastToFirstPersonCharacter (Game|GetPlayerCharacter 0)))
    (Variables|/Game/FirstPersonBP/Blueprints/FirstPersonCharacter.FirstPersonCharacter_C|SetTotal%20Coins _asfirst_person_character_2 (+ (Variables|/Game/FirstPersonBP/Blueprints/FirstPersonCharacter.FirstPersonCharacter_C|GetTotal%20Coins _asfirst_person_character_2) 5))
    (Utilities|FlowControl|Delay 7.0)
    (Actor|DestroyActor)
    (Variables|Default|SetisDead true)
    (else
      (Actor|DestroyActor _asfirst_person_projectile)
      (Variables|Default|SetisDead false))))

(fn ConstructionScript)