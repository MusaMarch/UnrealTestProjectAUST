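; BP_SaveGameSettings is a main menu data container, named as a save game, for screen resolution, shadow and texture quality settings.
; It keeps each option as both a command and a setting value, written together by SetSettings.
; ReturnCommand hands back the commands, while ReturnEnums hands back the matching setting values.
; It only stores values; applying them and saving to disk happen outside these graphs.
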(fn SetSettings
  (params (ScreenResCommand :type String) (ShadowCommand :type String) (TextureQualityCommand :type String) (ScreenSetting :type ENUM_Buttons%20Enum :default "NewEnumerator0") (ShadowSetting :type ENUM_Buttons%20Enum :default "NewEnumerator0") (TextureQualitySetting :type ENUM_Buttons%20Enum :default "NewEnumerator0"))
  (Variables|Default|SetScreenResCommand ScreenResCommand)
  (Variables|Default|SetShadowCommand ShadowCommand)
  (Variables|Default|SetTextureQualityCommand TextureQualityCommand)
  (Variables|Default|SetScreenSetting ScreenSetting)
  (Variables|Default|SetShadowSetting ShadowSetting)
  (Variables|Default|SetTextureQualitySetting TextureQualitySetting))

(fn ReturnCommand
  (return (Variables|Default|GetScreenResCommand) (Variables|Default|GetShadowCommand) (Variables|Default|GetTextureQualityCommand)))

(fn ReturnEnums
  (return (Variables|Default|GetScreenSetting) (Variables|Default|GetShadowSetting) (Variables|Default|GetTextureQualitySetting)))